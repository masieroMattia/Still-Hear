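; Player controller for StillHear that serves as a debug harness for input binding and rebinding.
; Tab toggles the keyboard binding widget, switching input mode and showing or hiding the cursor, while P flips the CommonInput gamepad type between PlayStation and Xbox.
; Number keys reset, save or delete bindings through the input subsystem.
; Unconnected test chains queue IA_Jump key swaps in either direction for RebindKeys and never run.
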(event Input|KeyboardEvents|1
  (params (Key :type Key%20Structure))
  ;[0.15 0.15 0.15 0.5] Input Rebinding Test
)

(event Input|KeyboardEvents|2
  (params (Key :type Key%20Structure))
  ;[0.15 0.15 0.15 0.5] Input Rebinding Test
)

(event Input|GamepadEvents|GamepadSpecialRight
  (params (Key :type Key%20Structure)))

(event Input|KeyboardEvents|3
  (params (Key :type Key%20Structure))
  ;[0.15 0.15 0.15 0.5] Input Rebinding Test
  (:Pressed
    (Class|InputSubsystem|ResetSavedBindingstoDefault (Subsystems|GetInputSubsystem))))

(event Input|KeyboardEvents|P
  (params (Key :type Key%20Structure))
  (:Pressed
    (Utilities|FlowControl|FlipFlop
      (:A
        (Class|CommonInputSubsystem|SetGamepadInputType (PlayerController|LocalPlayerSubsystems|GetCommonInputSubsystem) "PlayStation"))
      (:B
        (Class|CommonInputSubsystem|SetGamepadInputType (PlayerController|LocalPlayerSubsystems|GetCommonInputSubsystem) "Xbox")))))

(event Input|KeyboardEvents|0
  (params (Key :type Key%20Structure))
  ;[0.15 0.15 0.15 0.5] Input Rebinding Test
  (:Pressed
    (Class|InputSubsystem|SaveBindings (Subsystems|GetInputSubsystem))))

(event Input|KeyboardEvents|Tab
  (params (Key :type Key%20Structure))
  (:Pressed
    (Utilities|FlowControl|FlipFlop
      (:A
        (bind _returnvalue (UserInterface|CreateWidget "/Game/Programmers/Mattia/UI/Widgets/Menu/Settings/Controls/WBP_KeyboardBindingScreen.WBP_KeyboardBindingScreen_C" self))
        (bind _output_get (Variables|Default|Setcanvas _returnvalue))
        (UserInterface|Viewport|AddtoViewport _output_get 0)
        (Input|SetInputModeGameandUI self _output_get "DoNotLock" true false)
        (Variables|Default|SetbShowMouseCursor true))
      (:B
        (bind _canvas (Variables|Default|Getcanvas)
          (:then
            (Widget|RemovefromParent _canvas)
            (Input|SetInputModeGameOnly self false)
            (Variables|Default|SetbShowMouseCursor false))
          (:else))))))

(event Input|KeyboardEvents|9
  (params (Key :type Key%20Structure))
  ;[0.15 0.15 0.15 0.5] Input Rebinding Test
  (:Pressed
    (Class|InputSubsystem|DeleteBindings (Subsystems|GetInputSubsystem))))

(fn ConstructionScript)