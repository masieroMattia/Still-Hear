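; BP_Spawn is the spawn manager that creates and possesses the player's BP_StillHearMainCharacter.
; On BeginPlay, after a short delay, it spawns the character at LastPositionToSpawn and has player controller 0 possess it.
; An identity transform in LastPositionToSpawn counts as unset and falls back to StartingPoint.
; SetNewSpawnPoint stores a new position and priority unless that priority is lower than the current one.
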(event EventBeginPlay
  (Utilities|FlowControl|Delay 5.0)
  (if (== (Variables|Default|GetLastPositionToSpawn) (Math|Transform|MakeTransform "0, 0, 0"))
    (Variables|Default|SetLastPositionToSpawn (Variables|Default|GetStartingPoint)))
  (bind _returnvalue (Game|SpawnActorfromClass "/Game/Programmers/Edoardo/Characters/BP_StillHearMainCharacter.BP_StillHearMainCharacter_C" (Variables|Default|GetLastPositionToSpawn) "AdjustIfPossibleButAlwaysSpawn" "MultiplyWithRoot" 0 0))
  (Pawn|Possess (Game|GetPlayerController 0) _returnvalue))

(event Collision|EventActorBeginOverlap
  (params (OtherActor :type Actor%20Object%20Reference)))

(event EventTick
  (params (DeltaSeconds :type Float%20%28single-precision%29)))

(event EventOnPostLoad)

(fn ConstructionScript)

(fn SetNewSpawnPoint
  (params (Position :type Transform) (Priority :type Integer))
  (if (not (< Priority (Variables|Default|GetCurrentPriority)))
    (Variables|Default|SetLastPositionToSpawn Position)
    (Variables|Default|SetCurrentPriority Priority)))