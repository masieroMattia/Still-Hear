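; Checkpoint actor that moves the player spawn point forward when its trigger is overlapped.
; On overlap it passes its NextSpawnPoint location and Priority to the referenced spawner, then marks itself Completed.
; Completed checkpoints are hidden with collision and tick disabled, and OnPostLoad reapplies this state after loading.
; Overlaps are not filtered by actor, and debug prints trace each step.
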(event OnComponentBeginOverlap(Trigger)
  (params (OverlappedComponent :type Primitive%20Component%20Object%20Reference) (OtherActor :type Actor%20Object%20Reference) (OtherComp :type Primitive%20Component%20Object%20Reference) (OtherBodyIndex :type Integer) (bFromSweep :type Boolean) (SweepResult :type Hit%20Result%20Structure%20%28by%20ref%29))
  (CallFunction|ActivateCeckpoint)
  (Development|PrintString "try activate")
  (Variables|Default|SetCompleted true)
  (if (Variables|Default|GetCompleted)
    (Rendering|SetActorHiddenInGame true)
    (Collision|SetActorEnableCollision false)
    (Actor|Tick|SetActorTickEnabled false)
    (Development|PrintString "Completed")))

(event EventBeginPlay)

(event Collision|EventActorBeginOverlap
  (params (OtherActor :type Actor%20Object%20Reference)))

(event EventOnPostLoad
  (if (Variables|Default|GetCompleted)
    (Rendering|SetActorHiddenInGame true)
    (Collision|SetActorEnableCollision false)
    (Actor|Tick|SetActorTickEnabled false)
    (Development|PrintString "Completed")))

(fn ConstructionScript)

(fn ActivateCeckpoint
  (bind _spawnerreference (Variables|Default|GetSpawnerReference))
  (bind _nextspawnpoint (Variables|Default|GetNextSpawnPoint))
  (bind _returnvalue (Transformation|GetWorldLocation _nextspawnpoint))
  (Utilities|IsValid _spawnerreference
    (:Is%20Valid
      (Default|SetNewSpawnPoint _spawnerreference (Math|Transform|MakeTransform _returnvalue "0, 0, 0" "1.000000,1.000000,1.000000") (Variables|Default|GetPriority))
      (Development|PrintString "Setted")
      (Development|PrintString (Utilities|String|ToString(Vector) _returnvalue)))))