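; Checkpoint actor that saves the game on touch and puts the player back at its position after a load.
; Any overlap with its Sphere sets IsActivated, requests an async save of the current slot, then hides the Sphere and disables its overlap events.
; On OnPostLoad, every activated checkpoint disables overlaps again and teleports player pawn 0 to itself, without re-hiding the Sphere.
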(event OnComponentBeginOverlap(Sphere)
  (params (OverlappedComponent :type Primitive%20Component%20Object%20Reference) (OtherActor :type Actor%20Object%20Reference) (OtherComp :type Primitive%20Component%20Object%20Reference) (OtherBodyIndex :type Integer) (bFromSweep :type Boolean) (SweepResult :type Hit%20Result%20Structure%20%28by%20ref%29))
  (bind _returnvalue (Subsystems|GetSaveSubsystem))
  (Variables|Default|SetbIsActivated true)
  (Class|SaveSubsystem|RequestSaveSlotAsync _returnvalue (Class|SaveSubsystem|GetCurrentSlotSave _returnvalue))
  (Rendering|SetVisibility (Variables|Default|GetSphere) false false)
  (Variables|/Script/Engine.PrimitiveComponent|SetbGenerateOverlapEvents (Variables|Default|GetSphere) false))

(event EventBeginPlay)

(event Collision|EventActorBeginOverlap
  (params (OtherActor :type Actor%20Object%20Reference)))

(event EventTick
  (params (DeltaSeconds :type Float%20%28single-precision%29)))

(event EventOnPreSave)

(event EventOnPostLoad
  (if (Variables|Default|GetbIsActivated)
    (Variables|/Script/Engine.PrimitiveComponent|SetbGenerateOverlapEvents (Variables|Default|GetSphere) false)
    (Transformation|SetActorLocation (Game|Player|GetPlayerPawn 0) (Transformation|GetActorLocation) false true)))

(fn ConstructionScript)