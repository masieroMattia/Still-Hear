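; BP_Trap is a trap actor that makes the player's floating companion react when the player character comes near.
; Entering its proximity sphere disables auto-polling on the player's FloatingCompanionComponent and sets the companion state to Scared.
; Leaving the sphere re-enables auto-polling and sets the state to Happy.
; The Blueprint itself holds no damage or trigger logic beyond this companion reaction.
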(event OnComponentBeginOverlap(ProximitySphereComponent)
  (params (OverlappedComponent :type Primitive%20Component%20Object%20Reference) (OtherActor :type Actor%20Object%20Reference) (OtherComp :type Primitive%20Component%20Object%20Reference) (OtherBodyIndex :type Integer) (bFromSweep :type Boolean) (SweepResult :type Hit%20Result%20Structure%20%28by%20ref%29))
  (bind _returnvalue (Game|GetPlayerCharacter 0))
  (bind _returnvalue_2 (Actor|GetComponentbyClass _returnvalue "/Script/StillHear.FloatingCompanionComponent"))
  (if (== OtherActor _returnvalue)
    (Utilities|IsValid _returnvalue_2
      (:Is%20Valid
        (Class|FloatingCompanionComponent|SetAutoPollingEnabled _returnvalue_2 false)
        (Class|FloatingCompanionComponent|SetCompanionState _returnvalue_2 "Scared")))))

(event OnComponentEndOverlap(ProximitySphereComponent)
  (params (OverlappedComponent :type Primitive%20Component%20Object%20Reference) (OtherActor :type Actor%20Object%20Reference) (OtherComp :type Primitive%20Component%20Object%20Reference) (OtherBodyIndex :type Integer))
  (bind _returnvalue (Game|GetPlayerCharacter 0))
  (bind _returnvalue_2 (Actor|GetComponentbyClass _returnvalue "/Script/StillHear.FloatingCompanionComponent"))
  (if (== OtherActor _returnvalue)
    (Utilities|IsValid _returnvalue_2
      (:Is%20Valid
        (Class|FloatingCompanionComponent|SetAutoPollingEnabled _returnvalue_2 true)
        (Class|FloatingCompanionComponent|SetCompanionState _returnvalue_2 "Happy")))))

(event EventBeginPlay)

(fn ConstructionScript)