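; BP_RepeaterFlower is an interactable flower actor that reports a noise event tagged "Repeater" at its location whenever interaction stops.
; On BeginPlay it binds to the interaction-stopped event and freezes its animation in the open or closed pose based on StartOpen.
; Flowers that start closed then play the animation forward to open, wait OpenDuration, and play it in reverse to close.
; Flowers that start open only emit the noise.
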(event Custom|OnInteractionStopped_Event
  (bind _self self)
  (bind _skeletalmesh (Variables|Default|GetSkeletalMesh))
  (bind _skeletalmesh_2 (Variables|Default|GetSkeletalMesh))
  (Class|AISenseHearing|ReportNoiseEvent (Transformation|GetActorLocation _self) (Variables|Utils|GetLoudness) _self (Variables|Utils|GetMax%20Range) "Repeater")
  (if (not (Variables|Utils|GetbStartOpen))
    (Components|Animation|PlayAnimation _skeletalmesh "/Game/Artists/Veronica/mesh/assets/Repeater_Flower/Anim_Repeater_Flower.Anim_Repeater_Flower" false)
    (Components|Animation|SetPosition _skeletalmesh 0.0 false)
    (Components|Timeline|SetPlayRate _skeletalmesh 1.0)
    (Utilities|FlowControl|Delay (Variables|Utils|GetOpenDuration))
    (Components|Animation|PlayAnimation _skeletalmesh_2 "/Game/Artists/Veronica/mesh/assets/Repeater_Flower/Anim_Repeater_Flower.Anim_Repeater_Flower" false)
    (Components|Animation|SetPosition _skeletalmesh_2 2.0 false)
    (Components|Timeline|SetPlayRate _skeletalmesh_2 -1.0)))

(event EventBeginPlay
  (bind _skeletalmesh (Variables|Default|GetSkeletalMesh))
  (EventDispatchers|AssignOnInteractionStopped (delegate Custom|OnInteractionStopped_Event))
  (Components|Animation|PlayAnimation _skeletalmesh "/Game/Artists/Veronica/mesh/assets/Repeater_Flower/Anim_Repeater_Flower.Anim_Repeater_Flower" false)
  (Components|Timeline|SetPlayRate _skeletalmesh 0.0)
  (if (Variables|Utils|GetbStartOpen)
    (Components|Animation|SetPosition _skeletalmesh 2.0 false)
    (else
      (Components|Animation|SetPosition _skeletalmesh 0.0 false))))

(fn ConstructionScript)