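; BP_ResonanceWall is an interaction actor that plays collapse effects when triggered.
; On BeginPlay it binds its triggered event to StartVFX.
; After a short delay, StartVFX spawns a crystal dust Niagara system above the actor, plays a statue collapse sound and runs a camera shake preset through the camera effects.
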(event Custom|StartVFX
  (params (Triggerer :type Actor%20Object%20Reference))
  (Utilities|FlowControl|Delay 1.75)
  (Niagara|SpawnSystematLocation "/Game/Designers/Federico/Niagara/NS_DustCrystal.NS_DustCrystal" (+ (Transformation|GetActorLocation) "0.000000,0.000000,510.000000"))
  (Audio|PlaySoundatLocation "/Game/Designers/Federico/SoundTest/Rock/SFX_StatueCollapse_Cue.SFX_StatueCollapse_Cue" (Transformation|GetActorLocation) "0, 0, 0" 1.0 1.0 0.0 0 0 0 0)
  (Class|CameraEffectsComponent|PlayEffectPreset (Class|CameraEffectsBlueprintLibrary|GetCameraEffects) (Variables|Default|GetCamera%20shake%20preset)))

(event EventBeginPlay
  (EventDispatchers|BindEventtoOnTriggeredby (delegate Custom|StartVFX)))

(fn ConstructionScript)