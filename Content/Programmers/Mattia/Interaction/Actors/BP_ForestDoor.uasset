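; Forest door actor that reacts to interaction start and finish with a delayed Flow trigger and impact effects.
; On BeginPlay it binds both interaction events: the start waits briefly, then starts the root Flow graph from its Flow component.
; The finish spawns crystal dust and enlarged rock spark Niagara systems low on both sides, at fixed world-axis offsets that ignore door rotation.
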(event Custom|Start%20Shake
  (Utilities|FlowControl|Delay 2.0)
  (Class|FlowComponent|StartRootFlow (Variables|Default|GetFlow)))

(event Custom|Call%20VFX
  (Niagara|SpawnSystematLocation "/Game/Designers/Federico/Niagara/NS_DustCrystal.NS_DustCrystal" (+ (Transformation|GetActorLocation) "-480.000000,0.000000,-300.000000"))
  (Niagara|SpawnSystematLocation "/Game/Designers/Federico/Niagara/NS_RockSparks.NS_RockSparks" (+ (Transformation|GetActorLocation) "-480.000000,0.000000,-300.000000") "0, 0, 0" "3.000000,3.000000,3.000000")
  (Niagara|SpawnSystematLocation "/Game/Designers/Federico/Niagara/NS_DustCrystal.NS_DustCrystal" (+ (Transformation|GetActorLocation) "480.000000,0.000000,-300.000000"))
  (Niagara|SpawnSystematLocation "/Game/Designers/Federico/Niagara/NS_RockSparks.NS_RockSparks" (+ (Transformation|GetActorLocation) "480.000000,0.000000,-300.000000") "0, 0, 0" "3.000000,3.000000,3.000000"))

(event EventBeginPlay
  (EventDispatchers|BindEventtoOnInteractionStarted (delegate Custom|Start%20Shake))
  (EventDispatchers|BindEventtoOnInteractionFinished (delegate Custom|Call%20VFX)))

(fn ConstructionScript)