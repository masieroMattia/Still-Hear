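; BP_BellsStructure is an actor made of a structure and three bells that plays effects when an interaction starts.
; On BeginPlay it attaches the bells to the structure, keeping world location, and binds StartVFX to the interaction-started event.
; StartVFX spawns Niagara crystal dust and sparks at two stored locations, then plays a camera shake preset through the camera effects.
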(event Custom|StartVFX
  (Niagara|SpawnSystematLocation "/Game/Designers/Federico/Niagara/NS_DustCrystal.NS_DustCrystal" (Variables|Default|GetLocationD))
  (Niagara|SpawnSystematLocation "/Game/Designers/Federico/Niagara/NS_Sparks.NS_Sparks" (Variables|Default|GetLocationD))
  (Niagara|SpawnSystematLocation "/Game/Designers/Federico/Niagara/NS_Sparks.NS_Sparks" (Variables|Default|GetLocationA))
  (Class|CameraEffectsComponent|PlayEffectPreset (Class|CameraEffectsBlueprintLibrary|GetCameraEffects) (Variables|Default|GetCameraShake) "0, 0, 0"))

(event EventBeginPlay
  (Transformation|AttachComponentToComponent (Variables|Default|GetBell_01) (Variables|Default|GetStructure) "None" "KeepWorld" "KeepRelative" "KeepRelative" false)
  (Transformation|AttachComponentToComponent (Variables|Default|GetBell_02) (Variables|Default|GetStructure) "None" "KeepWorld" "KeepRelative" "KeepRelative" false)
  (Transformation|AttachComponentToComponent (Variables|Default|GetBell_03) (Variables|Default|GetStructure) "None" "KeepWorld" "KeepRelative" "KeepRelative" false)
  (EventDispatchers|BindEventtoOnInteractionStarted (delegate Custom|StartVFX)))

(fn ConstructionScript)