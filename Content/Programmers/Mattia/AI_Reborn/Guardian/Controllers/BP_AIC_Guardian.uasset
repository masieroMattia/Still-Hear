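; AI controller for the Guardian enemy that runs its behavior tree when it possesses a pawn.
; Its perception component listens for successfully sensed stimuli tagged "Repeater".
; Each one writes the stimulus location to the TargetLocation blackboard key, flattened to the pawn's own height so the tree gets a same-level target.
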(event OnTargetPerceptionUpdated(AIPerception)
  (params (Actor :type Actor%20Object%20Reference) (Stimulus :type AI%20Stimulus%20Structure))
  (bind (_x _y) (Math|Vector|BreakVector (.stimuluslocation Stimulus)))
  (bind _blackboard (Variables|Default|GetBlackboard))
  (if (.bsuccessfullysensed Stimulus)
    (if (== (.tag Stimulus) "Repeater")
      (Utilities|IsValid _blackboard
        (:Is%20Valid
          (AI|Components|Blackboard|SetValueasVector _blackboard (Utilities|Name|MakeLiteralName "TargetLocation") (Math|Vector|MakeVector _x _y (.Z (Math|Vector|BreakVector (Transformation|GetActorLocation (Pawn|GetControlledPawn self)))))))))))

(event EventPossess
  (params (PossessedPawn :type Pawn%20Object%20Reference))
  (AI|RunBehaviorTree "/Game/Programmers/Mattia/AI_Reborn/Guardian/BT/BT_Guardian.BT_Guardian"))

(fn ConstructionScript)