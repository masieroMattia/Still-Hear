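; BP_Guardian is a guardian character that automatically operates a designated lever when it comes within range.
; Its sphere overlap filters for LeverToTrigger, then runs a delayed sequence: engage the lever's interaction spot through CompanionComponent, trigger the interaction, and disengage.
; On post-load, the guardian destroys itself if LifeCameToTheEnd is set, so an expired guardian does not return after loading.
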(event OnComponentBeginOverlap(Sphere)
  (params (OverlappedComponent :type Primitive%20Component%20Object%20Reference) (OtherActor :type Actor%20Object%20Reference) (OtherComp :type Primitive%20Component%20Object%20Reference) (OtherBodyIndex :type Integer) (bFromSweep :type Boolean) (SweepResult :type Hit%20Result%20Structure%20%28by%20ref%29))
  (bind _levertotrigger (Variables|Default|GetLeverToTrigger))
  (if (== OtherActor _levertotrigger)
    (Utilities|FlowControl|Delay 1.0)
    (Class|FloatingCompanionComponent|EngageInteractionSpot (Variables|Default|GetCompanionComponent) (Actor|GetComponentbyClass _levertotrigger "/Script/StillHear.CompanionInteractionSpotComponent"))
    (Utilities|FlowControl|Delay 1.0)
    (Class|InteractableObj|TriggerInteraction _levertotrigger 0)
    (Utilities|FlowControl|Delay 1.0)
    (Class|FloatingCompanionComponent|DisengageInteractionSpot (Variables|Default|GetCompanionComponent))))

(event EventOnPostLoad
  (if (Variables|Default|GetLifeCameToTheEnd)
    (Actor|DestroyActor)))

(fn ConstructionScript)