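; A test player controller that drives the game UI through the UI subsystem's tagged widget layers.
; On possess it pushes the HUD onto the Game layer.
; The pause-toggle input pushes a tutorial input popup onto the Menu layer and initializes it with a message and input actions, including Activate Resonance and Parry.
; The pause menu push is left disconnected, so the pause key only opens the tutorial popup.
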(event Input|EnhancedActionEvents|EnhancedInputActionIA_TogglePause
  (params (ActionValue :type Boolean) (ElapsedSeconds :type Float%20%28double-precision%29) (TriggeredSeconds :type Float%20%28double-precision%29) (InputAction :type Input%20Action%20Object%20Reference :default "/Game/Programmers/Mattia/UI/Inputs/Actions/IA_TogglePause.IA_TogglePause"))
  (:Started
    (bind _returnvalue (Class|UISubsystem|PushWidgettoLayer (Subsystems|GetUISubsystem) "(TagName=\"UI.Layer.Menu\")" "/Game/Programmers/Mattia/UI/Widgets/Tutorial/WBP_TutorialInputPopup.WBP_TutorialInputPopup_C" false))
    (bind _aswbp_tutorial_input_popup (Utilities|Casting|CastToWBP_TutorialInputPopup _returnvalue))
    (Class|TutorialPopupWidget|InitializeTutorial _aswbp_tutorial_input_popup (Variables|Default|GetIn%20Message) (Utilities|Array|MakeArray "/Game/Programmers/Edoardo/Input/Actions/Ability/Resonance/IA_ActivateResonance.IA_ActivateResonance" "/Game/Programmers/Edoardo/Input/Actions/Ability/IA_Parry.IA_Parry" 0) 0.0)))

(event EventPossess
  (params (PossessedPawn :type Pawn%20Object%20Reference))
  (Class|UISubsystem|PushWidgettoLayer (Subsystems|GetUISubsystem) "(TagName=\"UI.Layer.Game\")" "/Game/Programmers/Mattia/UI/Widgets/HUD/WBP_HUD.WBP_HUD_C" false))

(fn ConstructionScript)