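; Player controller for the designers' game mode in StillHear, handling save feedback, pausing and a hidden key sequence.
; On possess it binds to the save subsystem to show a checkpoint widget when saving starts.
; The pause input pushes a game-pausing menu and sets cinematic pause until that widget deactivates.
; Key presses advance through a sequence that sets EGMount; debug shortcuts for time, abilities, bindings and graphics are left disconnected.
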(event Custom|CinematicUnpause
  (Class|StillHearPlayerController|SetCinematicPause false))

(event Custom|OnSaved
  (Class|UISubsystem|PushWidgettoLayer (Subsystems|GetUISubsystem) "(TagName=\"UI.Layer.Window\")" "/Game/Programmers/Mattia/UI/Widgets/HUD/WBP_Checpoint.WBP_Checpoint_C" true false))

(event Input|EnhancedActionEvents|EnhancedInputActionIA_TogglePause
  (params (ActionValue :type Boolean) (ElapsedSeconds :type Float%20%28double-precision%29) (TriggeredSeconds :type Float%20%28double-precision%29) (InputAction :type Input%20Action%20Object%20Reference :default "/Game/Programmers/Mattia/UI/Inputs/Actions/IA_TogglePause.IA_TogglePause"))
  (bind _returnvalue (Class|UISubsystem|PushWidgettoLayer (Subsystems|GetUISubsystem) "(TagName=\"UI.Layer.Menu\")" "/Game/Programmers/Mattia/UI/Widgets/Menu/PauseMenu/WBP_PauseMenu.WBP_PauseMenu_C" false true))
  (Class|StillHearPlayerController|SetCinematicPause true)
  (EventDispatchers|BindEventtoBPonWidgetDeactivated _returnvalue (delegate Custom|CinematicUnpause)))

(event EventPossess
  (params (PossessedPawn :type Pawn%20Object%20Reference))
  (EventDispatchers|BindEventtoOnSaveStarted (Subsystems|GetSaveSubsystem) (delegate Custom|OnSaved)))

(event Input|KeyboardEvents|0
  (params (Key :type Key%20Structure :default "None"))
  ;[0.149 0 0 0.502] DEBUG - Shortcut to reset binding - TO REMOVE
)

(event Input|KeyboardEvents|3
  (params (Key :type Key%20Structure :default "None"))
  ;[0.149 0 0 0.502] DEBUG - Shortcut to Manipulate Time - TO REMOVE
)

(event Input|KeyboardEvents|2
  (params (Key :type Key%20Structure :default "None"))
  ;[0.149 0 0 0.502] DEBUG - Shortcut to Manipulate Time - TO REMOVE
)

(event Input|KeyboardEvents|Period
  (params (Key :type Key%20Structure :default "None"))
  ;[0.149 0 0 0.502] DEBUG - Shortcut to Toggle Graphics Debug - TO REMOVE
)

(event Input|KeyboardEvents|1
  (params (Key :type Key%20Structure :default "None"))
  ;[0.149 0 0 0.502] DEBUG - Shortcut to Manipulate Time - TO REMOVE
)

(event Input|KeyboardEvents|Hyphen
  (params (Key :type Key%20Structure :default "None"))
  ;[0.149 0 0 0.502] DEBUG - Shortcut to give abilities - TO REMOVE
)

(event Input|KeyboardEvents|AnyKey
  (params (Key :type Key%20Structure :default "None"))
  ;[0.15 0.09592 0 0.5] SENSIBLE CODE
  (:Pressed
    (if (not (Variables|Default|GetEGMount))
      (if (== Key (Utilities|Array|Get(acopy) (Variables|Default|GetEGMountSequence) (Variables|Default|GetEGIndex)))
        (Math|Integer|IncrementInt (Variables|Default|GetEGIndex)
          (:%20%20
            (if (>= (Variables|Default|GetEGIndex) (- (Utilities|Array|Length (Variables|Default|GetEGMountSequence)) 1))
              (Variables|Default|SetEGMount true))))
        (else
          (Variables|Default|SetEGIndex 0))))))

(fn ConstructionScript)