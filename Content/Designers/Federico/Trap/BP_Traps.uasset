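; BP_Traps is a one-shot bear trap that catches and immobilizes the player character.
; The first box overlap by BP_DesignersStillHearMainCharacter stores the hit location, disables movement, plays the snap sound and the skeletal mesh's trap animation.
; A timeline then lerps player 0 to the box's center in X/Y at a fixed world Z.
; This Blueprint never resets the trap or restores movement.
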(event OnComponentBeginOverlap(Box)
  (params (OverlappedComponent :type Primitive%20Component%20Object%20Reference) (OtherActor :type Actor%20Object%20Reference) (OtherComp :type Primitive%20Component%20Object%20Reference) (OtherBodyIndex :type Integer) (bFromSweep :type Boolean) (SweepResult :type Hit%20Result%20Structure%20%28by%20ref%29))
  (bind _box (Variables|Default|GetBox))
  (bind _returnvalue (Transformation|GetWorldLocation _box))
  (bind _asbp_designers_still_hear_main_character (Utilities|Casting|CastToBP_DesignersStillHearMainCharacter OtherActor))
  (Utilities|FlowControl|DoOnce false
    (:Completed
      (Variables|Default|SetPlayerHitLocation (Transformation|GetActorLocation _asbp_designers_still_hear_main_character))
      (Pawn|Components|CharacterMovement|DisableMovement (Variables|/Script/Engine.Character|GetCharacterMovement _asbp_designers_still_hear_main_character))
      (Audio|PlaySoundatLocation "/Game/Designers/Federico/Trap/Sound/BearTrapSFX_Cue.BearTrapSFX_Cue" (Transformation|GetActorLocation) "0, 0, 0" 1.0 1.0 0.0 0 0 0 0)
      (Components|Animation|PlayAnimation (Variables|Default|GetSkeletalMesh) "/Game/Designers/Federico/Trap/source/AM_Trap.AM_Trap" false)
      ;[0.15 0.15 0.15 0.5] SnapPlayerToTrapCenter
      (bind _snaptocenter (Timeline|MovePlayeròToTrapCenter Play)
        (:Update
          (Transformation|SetActorLocation (Game|GetPlayerCharacter 0) (Math|Vector|Lerp(Vector) (Variables|Default|GetPlayerHitLocation) (Math|Vector|MakeVector (.x _returnvalue) (.y _returnvalue) 5e+01) _snaptocenter) false false))))))

(event EventBeginPlay)

(event Collision|EventActorBeginOverlap
  (params (OtherActor :type Actor%20Object%20Reference)))

(event EventTick
  (params (DeltaSeconds :type Float%20%28single-precision%29)))

(fn ConstructionScript)