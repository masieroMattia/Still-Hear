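; Scripted gate interactable that moves on curve-driven interactions and reacts to an intact crystal gate entering its box.
; That overlap spawns spark and dust effects, ends the interaction, plays a camera effect, then restarts after a delay with a faster backward rate.
; Each interaction start toggles GateUP; each finish spawns dust and, if GateUP is set, waits briefly before starting again at a slow backward rate.
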(event OnComponentBeginOverlap(Box)
  (params (OverlappedComponent :type Primitive%20Component%20Object%20Reference) (OtherActor :type Actor%20Object%20Reference) (OtherComp :type Primitive%20Component%20Object%20Reference) (OtherBodyIndex :type Integer) (bFromSweep :type Boolean) (SweepResult :type Hit%20Result%20Structure%20%28by%20ref%29))
  (bind _asbp_crystal_gate (Utilities|Casting|CastToBP_CrystalGate OtherActor))
  (switch Utilities|FlowControl|Switch|SwitchonEChaosResonanceState (Class|ChaosResonanceObj|GetResonanceState _asbp_crystal_gate)
    (:Intact
      (Niagara|SpawnSystematLocation "/Game/Designers/Federico/Niagara/NS_CrystalSparks.NS_CrystalSparks" (+ (Transformation|GetActorLocation _asbp_crystal_gate) "60.000000,0.000000,-100.000000"))
      (Niagara|SpawnSystematLocation "/Game/Designers/Federico/Niagara/NS_Sparks.NS_Sparks" (+ (Transformation|GetActorLocation _asbp_crystal_gate) "60.000000,0.000000,-100.000000"))
      (Niagara|SpawnSystematLocation "/Game/Designers/Federico/Niagara/NS_DustCrystal.NS_DustCrystal" (+ (Transformation|GetActorLocation _asbp_crystal_gate) "60.000000,0.000000,-100.000000"))
      (Class|InteractableObj|CallEndInteraction)
      (Class|CameraEffectsComponent|PlayEffectPreset (Class|CameraEffectsBlueprintLibrary|GetCameraEffects) (Variables|Default|GetCameraEffectsPreset) "0, 0, 0")
      (Utilities|FlowControl|Delay 2.0)
      (Variables|Default|SetBackwardCurveRate 1.3)
      (Class|InteractableObj|CallStartInteraction))))

(event Custom|G|ateTimer
  (Niagara|SpawnSystematLocation "/Game/Designers/Federico/Niagara/NS_DustCrystal.NS_DustCrystal" (Transformation|GetActorLocation))
  (if (Variables|Default|GetGateUP)
    (Utilities|FlowControl|Delay 1.0)
    (Variables|Default|SetBackwardCurveRate 0.07)
    (Class|InteractableObj|CallStartInteraction)))

(event Custom|GateUPstart
  (if (Variables|Default|GetGateUP)
    (Variables|Default|SetGateUP false)
    (else
      (Variables|Default|SetGateUP true))))

(event EventBeginPlay
  (Variables|Default|SetMeshLocation (Variables|/Script/Engine.SceneComponent|GetRelativeLocation (Variables|Default|GetGateMesh)))
  (EventDispatchers|BindEventtoOnInteractionStarted (delegate Custom|GateUPstart))
  (EventDispatchers|BindEventtoOnInteractionFinished (delegate Custom|G|ateTimer)))

(fn ConstructionScript)