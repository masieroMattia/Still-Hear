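; Interactable hanging bell that swings and, when interacted with, emits a very loud AI noise event tagged as a bell vibration.
; An Oscilla timeline starts on BeginPlay, driving the pitch of the chain and bell mesh.
; Interaction start is bound to Destroy, which despite its name reports the noise at the bell's location and plays a second timeline on the same rotations without stopping the first.
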(event Custom|Destroy
  (Class|AISenseHearing|ReportNoiseEvent (Transformation|GetActorLocation) 999.0 self 0.0 "Vibration.Bell")
  (bind _oscillator (Timeline|Timeline Play)
    (:Update
      (Transformation|SetRelativeRotation (Variables|Default|GetChain) (Math|Rotator|MakeRotator 0.0 _oscillator 0.0) false false)
      (Transformation|SetRelativeRotation (Variables|Default|GetStaticMeshComponent) (Math|Rotator|MakeRotator 0.0 (* _oscillator 1.0) 0.0) false false))))

(event EventBeginPlay
  (Utilities|FlowControl|Sequence
    (:then_0
      (bind _oscillator (Timeline|Oscilla Play)
        (:Update
          (Transformation|SetRelativeRotation (Variables|Default|GetChain) (Math|Rotator|MakeRotator 0.0 _oscillator 0.0) false false)
          (Transformation|SetRelativeRotation (Variables|Default|GetStaticMeshComponent) (Math|Rotator|MakeRotator 0.0 (* _oscillator 1.0) 0.0) false false))))
    (:then_1
      (EventDispatchers|BindEventtoOnInteractionStarted (delegate Custom|Destroy)))))

(fn ConstructionScript)