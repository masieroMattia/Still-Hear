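; BP_FallingRockN2 is a trigger-driven falling rock chaos actor with lighting effects, built around three overlap volumes.
; Box fires CallInteraction when the main character enters and applies a light function material to the PointLight.
; HideObj hides the SMGround06M mesh on player overlap, while DisableLight clears the light function and zeroes the light's intensity.
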(event OnComponentBeginOverlap(Box)
  (params (OverlappedComponent :type Primitive%20Component%20Object%20Reference) (OtherActor :type Actor%20Object%20Reference) (OtherComp :type Primitive%20Component%20Object%20Reference) (OtherBodyIndex :type Integer) (bFromSweep :type Boolean) (SweepResult :type Hit%20Result%20Structure%20%28by%20ref%29))
  (Utilities|Casting|CastToBP_DesignersStillHearMainCharacter OtherActor)
  (Class|ChaosResonanceObj|CallInteraction)
  (Rendering|Components|Light|SetLightFunctionMaterial (Variables|Default|GetPointLight) "/Game/Designers/Federico/Materials/M_LightFunction.M_LightFunction"))

(event OnComponentBeginOverlap(HideObj)
  (params (OverlappedComponent :type Primitive%20Component%20Object%20Reference) (OtherActor :type Actor%20Object%20Reference) (OtherComp :type Primitive%20Component%20Object%20Reference) (OtherBodyIndex :type Integer) (bFromSweep :type Boolean) (SweepResult :type Hit%20Result%20Structure%20%28by%20ref%29))
  (if (== (Game|GetPlayerCharacter 0) OtherActor)
    (Rendering|SetVisibility (Variables|Default|GetSM_Ground_06_m) false false)))

(event OnComponentBeginOverlap(DisableLight)
  (params (OverlappedComponent :type Primitive%20Component%20Object%20Reference) (OtherActor :type Actor%20Object%20Reference) (OtherComp :type Primitive%20Component%20Object%20Reference) (OtherBodyIndex :type Integer) (bFromSweep :type Boolean) (SweepResult :type Hit%20Result%20Structure%20%28by%20ref%29))
  (bind _pointlight (Variables|Default|GetPointLight))
  (if (== (Game|GetPlayerCharacter 0) OtherActor)
    (Rendering|Components|Light|SetLightFunctionMaterial _pointlight 0)
    (Rendering|Components|Light|SetIntensity _pointlight 0.0)))

(fn ConstructionScript)