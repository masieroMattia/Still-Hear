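; Falling rock Chaos actor that reacts to the player character entering two trigger volumes.
; TriggerFall calls CallInteraction, plays an initial camera shake preset and applies a light function material to the point light.
; TriggerCameraShake plays a second shake preset, clears that light function and turns the light's intensity to zero.
; The fall itself is not scripted in this graph.
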(event OnComponentBeginOverlap(TriggerFall)
  (params (OverlappedComponent :type Primitive%20Component%20Object%20Reference) (OtherActor :type Actor%20Object%20Reference) (OtherComp :type Primitive%20Component%20Object%20Reference) (OtherBodyIndex :type Integer) (bFromSweep :type Boolean) (SweepResult :type Hit%20Result%20Structure%20%28by%20ref%29))
  (if (== (Game|GetPlayerCharacter 0) OtherActor)
    (Class|ChaosResonanceObj|CallInteraction)
    (Class|CameraEffectsComponent|PlayEffectPreset (Class|CameraEffectsBlueprintLibrary|GetCameraEffects) (Variables|Default|GetCamera%20Effects%20Preset%20Shake%20Init) "0, 0, 0")
    (Rendering|Components|Light|SetLightFunctionMaterial (Variables|Default|GetPointLight) "/Game/Designers/Federico/Materials/M_LightFunction.M_LightFunction")))

(event OnComponentBeginOverlap(TriggerCameraShake)
  (params (OverlappedComponent :type Primitive%20Component%20Object%20Reference) (OtherActor :type Actor%20Object%20Reference) (OtherComp :type Primitive%20Component%20Object%20Reference) (OtherBodyIndex :type Integer) (bFromSweep :type Boolean) (SweepResult :type Hit%20Result%20Structure%20%28by%20ref%29))
  (bind _pointlight (Variables|Default|GetPointLight))
  (if (== (Game|GetPlayerCharacter 0) OtherActor)
    (Class|CameraEffectsComponent|PlayEffectPreset (Class|CameraEffectsBlueprintLibrary|GetCameraEffects) (Variables|Default|GetCamera%20Effects%20Preset%20Shake) "0, 0, 0")
    (Rendering|Components|Light|SetLightFunctionMaterial _pointlight 0)
    (Rendering|Components|Light|SetIntensity _pointlight 0.0)))

(fn ConstructionScript)