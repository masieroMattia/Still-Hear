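; BP_OpeningWall is an interactable wall that adds camera effects and crystal dust to its movement.
; BeginPlay binds its handlers to the interaction started and finished events, each guarded by a DoOnce.
; The first start plays a camera preset and spawns Niagara dust at the actor's location.
; The first finish restarts the interaction, plays the "UP" camera preset and spawns dust above the actor.
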(event Custom|Restart
  (Utilities|FlowControl|DoOnce false
    (:Completed
      (Class|InteractableObj|CallStartInteraction)
      (Class|CameraEffectsComponent|PlayEffectPreset (Class|CameraEffectsBlueprintLibrary|GetCameraEffects) (Variables|Default|GetCameraEffectsUP))
      (Niagara|SpawnSystematLocation "/Game/Designers/Federico/Niagara/NS_DustCrystal.NS_DustCrystal" (+ (Transformation|GetActorLocation) "0.000000,0.000000,450.000000")))))

(event Custom|Start%20effects
  (Utilities|FlowControl|DoOnce false
    (:Completed
      (Class|CameraEffectsComponent|PlayEffectPreset (Class|CameraEffectsBlueprintLibrary|GetCameraEffects) (Variables|Default|GetCameraEffects))
      (Niagara|SpawnSystematLocation "/Game/Designers/Federico/Niagara/NS_DustCrystal.NS_DustCrystal" (Transformation|GetActorLocation)))))

(event EventBeginPlay
  (EventDispatchers|BindEventtoOnInteractionFinished (delegate Custom|Restart))
  (EventDispatchers|BindEventtoOnInteractionStarted (delegate Custom|Start%20effects)))

(fn ConstructionScript)