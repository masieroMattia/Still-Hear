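; BP_Bell is a bell actor that swings and emits noise when its AddForce event fires.
; The event applies a velocity-change impulse to the Bell component and reports a loud noise event tagged "Vibration.Bell" at the actor's location.
; A timeline-driven wind sway and a binding of the event to a lever reference's AddForce dispatcher exist but are disconnected, and BeginPlay is empty.
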(event Custom|AddForce_Event
  (Physics|AddImpulse (Variables|Default|GetBell) "145.000000,0.000000,0.000000" "None" true)
  (Class|AISenseHearing|ReportNoiseEvent (Transformation|GetActorLocation) 5.0 self 0.0 "Vibration.Bell"))

(event EventBeginPlay)

(fn ConstructionScript)