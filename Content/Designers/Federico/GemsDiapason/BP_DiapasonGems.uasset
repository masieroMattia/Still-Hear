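; BP_DiapasonGems is a gem that shows its active state by swapping the material on its mesh, tied to a referenced door.
; ChangeMaterialActive applies a blue unlit glass material, then uses a retriggerable delay to restore the base blue metal material unless the door is open.
; Two helper functions, ChangeMaterial and ChangeMaterialOFF, apply a caller-supplied on or off material directly.
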(event Custom|ChangeMaterialActive
  (bind _gem (Variables|Default|GetGem))
  (bind _gem_2 (Variables|Default|GetGem))
  (Utilities|IsValid _gem_2
    (:Is%20Valid
      (Rendering|Material|SetMaterial _gem_2 0 "/Game/Programmers/Piero/Material/GlassUnlit/M_GlassUnlit_Blu.M_GlassUnlit_Blu")
      (Utilities|FlowControl|RetriggerableDelay 1.3)
      (if (not (Variables|/Game/Designers/Federico/Diapason/BP_DoorTemple.BP_DoorTemple_C|GetDoorOpen (Variables|Default|GetDoorRef)))
        (Utilities|IsValid _gem
          (:Is%20Valid
            (Rendering|Material|SetMaterial _gem 0 "/Engine/TemplateResources/MI_Template_BaseBlue_Metal.MI_Template_BaseBlue_Metal")))))))

(event EventBeginPlay)

(fn ConstructionScript)

(fn ChangeMaterial
  (params (Material%20 :type Material%20Interface%20Object%20Reference) (OffMaterial :type Material%20Interface%20Object%20Reference))
  (Rendering|Material|SetMaterial (Variables|Default|GetGem) 0 Material%20))

(fn ChangeMaterialOFF
  (params (Material%20 :type Material%20Interface%20Object%20Reference) (OffMaterial :type Material%20Interface%20Object%20Reference))
  (Rendering|Material|SetMaterial (Variables|Default|GetGem) 0 OffMaterial))