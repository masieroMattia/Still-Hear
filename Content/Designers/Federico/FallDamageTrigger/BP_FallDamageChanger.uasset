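; Trigger volume that temporarily changes the player character's fall damage setting while it is inside the box.
; Begin overlap sends a much higher value through UpdateFallDamageMessage and sets a Triggered flag, which this graph never reads.
; End overlap sends a far lower, hardcoded value, then disables the box's collision after a short delay, retiring the trigger.
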(event OnComponentBeginOverlap(Box)
  (params (OverlappedComponent :type Primitive%20Component%20Object%20Reference) (OtherActor :type Actor%20Object%20Reference) (OtherComp :type Primitive%20Component%20Object%20Reference) (OtherBodyIndex :type Integer) (bFromSweep :type Boolean) (SweepResult :type Hit%20Result%20Structure%20%28by%20ref%29))
  (if (== (Game|GetPlayerCharacter 0) OtherActor)
    (Class|BPIFallDamageChange|UpdateFallDamage(Message) OtherActor 9e+04)
    (Variables|Default|SetbTriggered true)))

(event OnComponentEndOverlap(Box)
  (params (OverlappedComponent :type Primitive%20Component%20Object%20Reference) (OtherActor :type Actor%20Object%20Reference) (OtherComp :type Primitive%20Component%20Object%20Reference) (OtherBodyIndex :type Integer))
  (if (== (Game|GetPlayerCharacter 0) OtherActor)
    (Class|BPIFallDamageChange|UpdateFallDamage(Message) OtherActor 6e+02)
    (Utilities|FlowControl|Delay 5.0)
    (Collision|SetCollisionEnabled (Variables|Default|GetBox) "NoCollision")))

(fn ConstructionScript)