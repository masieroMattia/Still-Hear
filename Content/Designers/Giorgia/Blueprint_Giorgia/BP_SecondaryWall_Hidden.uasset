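; BP_SecondaryWall_Hidden is a wall actor that hides itself while the player is inside its trigger area.
; When player character 0 begins overlapping TriggerEnter, both static mesh components are set hidden in game.
; When the player begins overlapping the separate TriggerExit, both meshes are shown again, so visibility depends on which trigger was entered last rather than on end-overlap events.
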(event OnComponentBeginOverlap(TriggerEnter)
  (params (OverlappedComponent :type Primitive%20Component%20Object%20Reference) (OtherActor :type Actor%20Object%20Reference) (OtherComp :type Primitive%20Component%20Object%20Reference) (OtherBodyIndex :type Integer) (bFromSweep :type Boolean) (SweepResult :type Hit%20Result%20Structure%20%28by%20ref%29))
  (if (== (Game|GetPlayerCharacter 0) OtherActor)
    (Development|SetHiddeninGame (Variables|Debug|GetStaticMeshComponent) true false)))

(event OnComponentBeginOverlap(TriggerExit)
  (params (OverlappedComponent :type Primitive%20Component%20Object%20Reference) (OtherActor :type Actor%20Object%20Reference) (OtherComp :type Primitive%20Component%20Object%20Reference) (OtherBodyIndex :type Integer) (bFromSweep :type Boolean) (SweepResult :type Hit%20Result%20Structure%20%28by%20ref%29))
  (if (== (Game|GetPlayerCharacter 0) OtherActor)
    (Development|SetHiddeninGame (Variables|Debug|GetStaticMeshComponent) false false)))

(fn ConstructionScript)