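; A trigger actor that drops six cones one after another when the player character enters its box.
; The box overlap fires FallingCone, which enables gravity on all six cone components at once.
; It then turns on physics simulation for each cone in sequence, separated by a shared Duration delay, creating a staggered fall.
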(event OnComponentBeginOverlap(Box)
  (params (OverlappedComponent :type Primitive%20Component%20Object%20Reference) (OtherActor :type Actor%20Object%20Reference) (OtherComp :type Primitive%20Component%20Object%20Reference) (OtherBodyIndex :type Integer) (bFromSweep :type Boolean) (SweepResult :type Hit%20Result%20Structure%20%28by%20ref%29))
  (if (== (Game|GetPlayerCharacter 0) OtherActor)
    (CallFunction|FallingCone)))

(event Custom|FallingCone
  (Physics|SetEnableGravity (Variables|Default|GetCone1) true)
  (Utilities|FlowControl|Delay (Variables|Default|GetDuration))
  (Physics|SetSimulatePhysics (Variables|Default|GetCone1) true)
  (Utilities|FlowControl|Delay (Variables|Default|GetDuration))
  (Physics|SetSimulatePhysics (Variables|Default|GetCone2) true)
  (Utilities|FlowControl|Delay (Variables|Default|GetDuration))
  (Physics|SetSimulatePhysics (Variables|Default|GetCone3) true)
  (Utilities|FlowControl|Delay (Variables|Default|GetDuration))
  (Physics|SetSimulatePhysics (Variables|Default|GetCone4) true)
  (Utilities|FlowControl|Delay (Variables|Default|GetDuration))
  (Physics|SetSimulatePhysics (Variables|Default|GetCone5) true)
  (Utilities|FlowControl|Delay (Variables|Default|GetDuration))
  (Physics|SetSimulatePhysics (Variables|Default|GetCone6) true))

(fn ConstructionScript)