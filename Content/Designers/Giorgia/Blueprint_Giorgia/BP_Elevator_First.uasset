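; Elevator actor that reacts to an interaction with an emissive glow and toggles a set of collision boxes around it.
; The player entering its sphere enables the boxes, and the interaction finishing disables them.
; Interaction start chains timelines that flare the Elevator material's Emissive Multiplier, settle it, then run a subtler glow.
; Interaction finish stops that glow and fades the emissive to zero.
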(event OnComponentBeginOverlap(SphereComponent)
  (params (OverlappedComponent :type Primitive%20Component%20Object%20Reference) (OtherActor :type Actor%20Object%20Reference) (OtherComp :type Primitive%20Component%20Object%20Reference) (OtherBodyIndex :type Integer) (bFromSweep :type Boolean) (SweepResult :type Hit%20Result%20Structure%20%28by%20ref%29))
  (if (== (Game|GetPlayerCharacter 0) OtherActor)
    (Collision|SetCollisionEnabled (Variables|Default|GetCollision) "QueryAndPhysics")))

(event Custom|EnableGlow
  (bind _glow (Timeline|Timeline Play)
    (:Update
      (Rendering|Material|SetScalarParameterValueonMaterials (Variables|Default|GetElevator) "Emissive Multiplier" (Math|Float|Lerp 0.0 6e+01 _glow)))
    (:Finished
      (bind _glow_2 (Timeline|Timeline_0 Play)
        (:Update
          (Rendering|Material|SetScalarParameterValueonMaterials (Variables|Default|GetElevator) "Emissive Multiplier" (Math|Float|Lerp 6e+01 1.0 _glow_2)))
        (:Finished
          (bind _glow_3 (Timeline|Timeline_2 Play)
            (:Update
              (Rendering|Material|SetScalarParameterValueonMaterials (Variables|Default|GetElevator) "Emissive Multiplier" (Math|Float|Lerp 1.0 5.0 _glow_3)))))))))

(event Custom|InteractionFinished
  (Collision|SetCollisionEnabled (Variables|Default|GetCollision) "NoCollision")
  (Utilities|FlowControl|Sequence
    (:then_0
      (bind _glow (Timeline|Timeline_2 Stop)
        (:Update
          (Rendering|Material|SetScalarParameterValueonMaterials (Variables|Default|GetElevator) "Emissive Multiplier" (Math|Float|Lerp 1.0 5.0 _glow)))))
    (:then_1
      (bind _glow_2 (Timeline|Timeline_1 Play)
        (:Update
          (Rendering|Material|SetScalarParameterValueonMaterials (Variables|Default|GetElevator) "Emissive Multiplier" (Math|Float|Lerp 5.0 0.0 _glow_2)))))))

(event EventBeginPlay
  (EventDispatchers|BindEventtoOnInteractionFinished (delegate Custom|InteractionFinished))
  (EventDispatchers|BindEventtoOnInteractionStarted (delegate Custom|EnableGlow)))

(fn ConstructionScript)