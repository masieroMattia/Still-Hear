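; BP_Elevator_Second is an elevator that runs a level sequence when the player character enters its trigger.
; After a short delay it enables collision on a set of box components and plays the referenced sequence.
; When the sequence finishes, a bound event switches those boxes back to no collision, so they block only during the ride.
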(event OnComponentBeginOverlap(Trigger)
  (params (OverlappedComponent :type Primitive%20Component%20Object%20Reference) (OtherActor :type Actor%20Object%20Reference) (OtherComp :type Primitive%20Component%20Object%20Reference) (OtherBodyIndex :type Integer) (bFromSweep :type Boolean) (SweepResult :type Hit%20Result%20Structure%20%28by%20ref%29))
  (bind _animreference (Variables|Default|GetAnimReference))
  (bind _sequenceplayer (Variables|/Script/LevelSequence.LevelSequenceActor|GetSequencePlayer _animreference))
  (if (== (Game|GetPlayerCharacter 0) OtherActor)
    (Utilities|FlowControl|Delay 2.0)
    (Collision|SetCollisionEnabled (Variables|Default|GetBox1) "QueryAndPhysics")
    (Sequencer|Player|Play _sequenceplayer :!class /Script/MovieScene.MovieSceneSequencePlayer)
    (EventDispatchers|AssignOnFinished _sequenceplayer (delegate Custom|OnFinished_Event))))

(event Custom|OnFinished_Event
  (Collision|SetCollisionEnabled (Variables|Default|GetBox1) "NoCollision"))

(fn ConstructionScript)